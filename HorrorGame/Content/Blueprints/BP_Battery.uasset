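; Battery pickup that recharges the player's battery when interacted with, then destroys itself.
; OnInteract adds Charge to the ThirdPersonCharacter's Baterry variable, or sets it straight to full when it is already near the cap.
; A Collision overlap shows the interaction prompt for the player character.
; A separate Highlight overlap, unfiltered by actor, toggles custom depth rendering on the Cylinder to highlight it.
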(event `/Game/Blueprints/Library/BP_Interaction.OnInteract`
  ;[0 0.3906 1] Adds more battery to the player
  (bind _asthird_person_character (cast `/Game/ThirdPersonBP/Blueprints/ThirdPersonCharacter` (`GameplayStatics.GetPlayerPawn` 0)))
  (bind _baterry (`/Game/ThirdPersonBP/Blueprints/ThirdPersonCharacter.Baterry` _asthird_person_character))
  (if (>= _baterry 90.0)
    (set `/Game/ThirdPersonBP/Blueprints/ThirdPersonCharacter.Baterry` 100.0 _asthird_person_character)
    (`self.K2_DestroyActor`)
    (else
      (set `/Game/ThirdPersonBP/Blueprints/ThirdPersonCharacter.Baterry` (+ _baterry (`self.Charge`)) _asthird_person_character)
      (`self.K2_DestroyActor`))))

(event `self.Collision.OnComponentBeginOverlap`
  (params (OverlappedComponent :type "PrimitiveComponent Object Reference") (OtherActor :type "Actor Object Reference") (OtherComp :type "PrimitiveComponent Object Reference") (OtherBodyIndex :type Integer) (bFromSweep :type Boolean) (SweepResult :type "HitResult Structure (by ref)"))
  ;[0 1 0.25] Ui to interact shows up
  (cast `/Game/ThirdPersonBP/Blueprints/ThirdPersonCharacter` OtherActor)
  (`SceneComponent.SetVisibility` (`self.InteractionInstruction`) true false))

(event `self.Highlight.OnComponentBeginOverlap`
  (params (OverlappedComponent :type "PrimitiveComponent Object Reference") (OtherActor :type "Actor Object Reference") (OtherComp :type "PrimitiveComponent Object Reference") (OtherBodyIndex :type Integer) (bFromSweep :type Boolean) (SweepResult :type "HitResult Structure (by ref)"))
  ;[0 0.3203 1] Highlight Object
  (`PrimitiveComponent.SetRenderCustomDepth` (`self.Cylinder`) true))

(event `self.Collision.OnComponentEndOverlap`
  (params (OverlappedComponent :type "PrimitiveComponent Object Reference") (OtherActor :type "Actor Object Reference") (OtherComp :type "PrimitiveComponent Object Reference") (OtherBodyIndex :type Integer))
  ;[0 1 0.25] Ui to interact shows up
  (`SceneComponent.SetVisibility` (`self.InteractionInstruction`) false false))

(event `self.Highlight.OnComponentEndOverlap`
  (params (OverlappedComponent :type "PrimitiveComponent Object Reference") (OtherActor :type "Actor Object Reference") (OtherComp :type "PrimitiveComponent Object Reference") (OtherBodyIndex :type Integer))
  (`PrimitiveComponent.SetRenderCustomDepth` (`self.Cylinder`) false))

(fn `UserConstructionScript`)